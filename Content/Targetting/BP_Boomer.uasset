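; BP_Boomer is a targetable actor that spawns an explosion below itself and is destroyed on a Sphere hit or Explosion event.
; InterfaceTargeting plays a timeline-driven widget animation, reset if targeting stops early.
; On completion it locks in, revealing the icon, cone and location/length widget, adding an identify widget and messaging the player pawn.
; An L-toggled Tick gate keeps WidgetDiserted hidden and yawed toward the camera.
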(event `self.Sphere.OnComponentHit`
  (params (HitComponent :type "PrimitiveComponent Object Reference") (OtherActor :type "Actor Object Reference") (OtherComp :type "PrimitiveComponent Object Reference") (NormalImpulse :type "Vector Structure") (Hit :type "HitResult Structure (by ref)"))
  (bind _returnvalue (`KismetMathLibrary.Conv_VectorToTransform` (`self.K2_GetActorLocation`)))
  (`|SpawnActorFromClass` "/Game/StarterContent/Blueprints/Blueprint_Effect_Explosion.Blueprint_Effect_Explosion_C" (`KismetMathLibrary.MakeTransform` (`KismetMathLibrary.MakeVector` (.x (.location _returnvalue)) (.y (.location _returnvalue)) (- (.z (.location _returnvalue)) 600.0))) "AdjustIfPossibleButAlwaysSpawn" "MultiplyWithRoot" null null)
  (`self.K2_DestroyActor`))

(event `/Game/Targetting/IF_Explosion.explosion`
  (bind _returnvalue (`KismetMathLibrary.Conv_VectorToTransform` (`self.K2_GetActorLocation`)))
  (`|SpawnActorFromClass` "/Game/StarterContent/Blueprints/Blueprint_Effect_Explosion.Blueprint_Effect_Explosion_C" (`KismetMathLibrary.MakeTransform` (`KismetMathLibrary.MakeVector` (.x (.location _returnvalue)) (.y (.location _returnvalue)) (- (.z (.location _returnvalue)) 600.0))) "AdjustIfPossibleButAlwaysSpawn" "MultiplyWithRoot" null null)
  (`self.K2_DestroyActor`))

(event `self.ReceiveTick`
  (params (DeltaSeconds :type "Float (single-precision)"))
  (bind _widget_diserted_ (`self.Widget(diserted)`))
  (bind (_returnvalue_roll _returnvalue_pitch _returnvalue_yaw) (`KismetMathLibrary.BreakRotator` (`KismetMathLibrary.FindLookAtRotation` (`SceneComponent.K2_GetComponentLocation` (`self.Widget(diserted)`)) (`self.K2_GetActorLocation` (`GameplayStatics.GetPlayerCameraManager` 0)))))
  (`/Engine/EditorBlueprintResources/StandardMacros.Gate` false :!label _label
    (:`Exit`
      (if false
        (`SceneComponent.SetVisibility` _widget_diserted_ true false)
        (else
          (`SceneComponent.SetVisibility` _widget_diserted_ false false)))
      (`SceneComponent.K2_SetWorldRotation` _widget_diserted_ (`KismetMathLibrary.MakeRotator` 0.0 0.0 _returnvalue_yaw) false false))))

(event `Key|L`
  (params (Key :type "Key Structure"))
  (:`Pressed`
    (goto _label :!via `Toggle`)))

(event `/Game/Targetting/BI_Targeting.InterfaceTargeting`
  (params (bContinueTargeting :type Boolean))
  (if (`self.bAnimationCompleted?`)
    _
    (elif bContinueTargeting
      (`SceneComponent.SetVisibility` (`self.Animation`) true false)
      (bind (_direction _alpha) (`Timeline|TargetingAnimation` :!label _label_2)
        (:`Update`
          (`/Game/Targetting/WG_TargetingAnimation.CE_TargetingAnimation` (`self.WG Targeting Animation`) _alpha))
        (:`Finished`
          (set `self.bAnimationCompleted?` true)
          (`|ExecutionSequence`
            (:`then_0`
              (`SceneComponent.SetVisibility` (`self.StaticIcon`) true false)
              (`/Game/Targetting/WG_TargetingIcon.CE_TargetingIcon` (`self.WG Targeting Icon`))
              (`|ExecutionSequence`
                (:`then_0`
                  (bind _returnvalue (`|GenericCreateObject` "/Game/Targetting/WG_BoomerIdentify.WG_BoomerIdentify_C"))
                  (`UserWidget.AddToViewport` _returnvalue 0)
                  (`SceneComponent.SetVisibility` (`self.Cone`) true false))
                (:`then_1`
                  (`/Game/Targetting/WG_LocationAndLength.CE_Length` (`self.WG Location And Length`) (`self.K2_GetActorLocation`))
                  (`SceneComponent.SetVisibility` (`self.LocationAndLength`) true false))
                (:`then_2`
                  (message `/Game/Targetting/Boomer_+1.Boomer_+1` (`GameplayStatics.GetPlayerPawn` 0))))))))
      (else
        (`|ExecutionSequence`
          (:`then_0`
            (goto _label_2 :!via `Stop`))
          (:`then_1`
            (goto _label_2 :!via `SetNewTime`))
          (:`then_2`
            (`SceneComponent.SetVisibility` (`self.Animation`) false false)))))))

(event `self.ReceiveBeginPlay`
  (`|ExecutionSequence`
    (:`then_1`
      (bind _aswg_targeting_animation (cast `/Game/Targetting/WG_TargetingAnimation` (`WidgetComponent.GetUserWidgetObject` (`self.Animation`))))
      (set `self.WG Targeting Animation` _aswg_targeting_animation)
      (bind _aswg_targeting_icon (cast `/Game/Targetting/WG_TargetingIcon` (`WidgetComponent.GetUserWidgetObject` (`self.StaticIcon`))))
      (set `self.WG Targeting Icon` _aswg_targeting_icon)
      (bind _aswg_location_and_length (cast `/Game/Targetting/WG_LocationAndLength` (`WidgetComponent.GetUserWidgetObject` (`self.LocationAndLength`))))
      (set `self.WG Location And Length` _aswg_location_and_length))))

(fn `UserConstructionScript`)