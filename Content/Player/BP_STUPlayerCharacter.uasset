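; Player character Blueprint that adds a first-person camera toggle on key 1 and a telescope targeting mode available in that view.
; The Telescope input toggles a delayed overlay widget and a fast timer that box-traces far ahead from the first-person camera.
; Hit actors implementing BI_Targeting receive targeting messages, with the current target tracked by object name and cleared when it changes or is lost.
; The overlay is hidden when the character is destroyed.
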(event `Key|One`
  (params (Key :type "Key Structure"))
  (bind _cameracomponent (`self.CameraComponent`))
  (:`Pressed`
    (`/Engine/EditorBlueprintResources/StandardMacros.FlipFlop`
      (:`A`
        (set `self.IfFirstCharacterView` true)
        (`ActorComponent.SetActive` _cameracomponent false false))
      (:`B`
        (set `self.IfFirstCharacterView` false)
        (`Widget.RemoveFromParent` (`self.WG_Telescope`))
        (`ActorComponent.SetActive` _cameracomponent true false)))
    (`SceneComponent.K2_SetRelativeRotation` (`self.SpringArmComponent`) (`self.K2_GetActorRotation` (`self.GetController`)) false false)))

(event `InputAction|Telescope`
  (params (Key :type "Key Structure"))
  (:`Pressed`
    (if (`self.IfFirstCharacterView`)
      (bind _isa (`/Engine/EditorBlueprintResources/StandardMacros.FlipFlop`)
        (:`A`
          _)
        (:`B`
          _))
      (`self.CE_Telescope` _isa)
      (if (`self.IfFirstCharacterView`)
        (bind _output_get (set `self.Telescope Mode Targeting` _isa))
        (`KismetSystemLibrary.K2_SetTimerDelegate` (delegate `CE_Targeting`) 0.01 _output_get)
        (else
          (`Widget.RemoveFromParent` (`self.WG_Telescope`)))))))

(event `CE_Targeting`
  (bind _firstcharactercamera (`self.FirstCharacterCamera`))
  (bind _returnvalue (`SceneComponent.K2_GetComponentLocation` _firstcharactercamera))
  (bind _outhit (`KismetSystemLibrary.BoxTraceSingle` _returnvalue (+ _returnvalue (* (`SceneComponent.GetForwardVector` _firstcharactercamera) 25000.0)) (80.0 80.0 80.0) (struct) "TraceTypeQuery1"))
  (if (`KismetStringLibrary.EqualEqual_StrStr` (`self.Fstring Primary Object Name`))
    (bind (_bblockinghit _binitialoverlap _time _distance _location _impactpoint _normal _impactnormal _physmat _hitactor) (`GameplayStatics.BreakHitResult` _outhit))
    (if (`KismetSystemLibrary.DoesImplementInterface` _hitactor "/Game/Targetting/BI_Targeting.BI_Targeting_C")
      (`|ExecutionSequence`
        (:`then_0`
          (bind _output_get (set `self.APrimary Actor` _hitactor))
          (set `self.Fstring Primary Object Name` (`KismetSystemLibrary.GetObjectName` _output_get)))
        (:`then_1`
          (`|ExecutionSequence`
            (:`then_0`
              _))))
      (message `/Game/Targetting/BI_Targeting.InterfaceTargeting` (`self.APrimary Actor`) (`self.Telescope Mode Targeting`) :!label _label))
    (elif (`KismetSystemLibrary.DoesImplementInterface` _hitactor "/Game/Targetting/BI_Targeting.BI_Targeting_C")
      (if (`KismetStringLibrary.EqualEqual_StrStr` (`KismetSystemLibrary.GetObjectName` _hitactor) (`self.Fstring Primary Object Name`))
        (goto _label)
        (else
          (message `/Game/Targetting/BI_Targeting.InterfaceTargeting` (`self.APrimary Actor`) false)
          (bind _output_get_2 (set `self.APrimary Actor` _hitactor))
          (set `self.Fstring Primary Object Name` (`KismetSystemLibrary.GetObjectName` _output_get_2))
          (goto _label)))
      (else
        (message `/Game/Targetting/BI_Targeting.InterfaceTargeting` (`self.APrimary Actor`) false)
        (set `self.Fstring Primary Object Name` "")
        (set `self.APrimary Actor` null)))))

(event `CE_Telescope`
  (params (bTelescoping :type Boolean))
  (bind _wg_telescope (`self.WG_Telescope`))
  (if bTelescoping
    (`KismetSystemLibrary.Delay` 0.2)
    (`UserWidget.AddToViewport` _wg_telescope 0)
    (else
      (`KismetSystemLibrary.Delay` 0.2)
      (`Widget.RemoveFromParent` _wg_telescope))))

(event `self.ReceiveBeginPlay`
  (`|ExecutionSequence`
    (:`then_1`
      (bind _returnvalue (`|CreateWidget` "/Game/Targetting/WG_Telescope.WG_Telescope_C"))
      (bind _output_get (set `self.WG_Telescope` _returnvalue))
      (add `self.OnDestroyed` (delegate `OnDestroyed_Event`)))))

(event `OnDestroyed_Event` :!signature `self.OnDestroyed`
  (params (DestroyedActor :type "Actor Object Reference"))
  (bind _output_get (set `self.IsDead` true))
  (if _output_get
    (`Widget.SetVisibility` (stale `self.ReceiveBeginPlay` _output_get) "Hidden")))

(fn `UserConstructionScript`)